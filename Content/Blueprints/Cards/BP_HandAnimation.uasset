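; Hand component that lays out drawn cards in a centered row relative to its owner and handles dragging them to play.
; OnDrawCard attaches and slots each card, snaps the layout, and binds the player controller's touch dispatcher events on every draw.
; Dragging projects the mouse position onto an owner-facing plane with a Z offset.
; On release, an applicable card is applied and removed before re-layout; otherwise it eases back to its slot.
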(event Custom|CustomEvent
  (params (actor :type Actor%20Object%20Reference) (location :type Vector) (screenPosition :type Vector%202D%20Structure))
  (bind _ascard (Utilities|Casting|CastToCard actor))
  (CallFunction|CardMoveHandler _ascard)
  (Variables|Default|SetDraggingCard _ascard)
  (Variables|Default|SetbDragging true))

(event Custom|CustomEvent_0
  (params (location :type Vector) (screenPosition :type Vector%202D%20Structure))
  (if (Variables|Default|GetbDragging)
    (CallFunction|CardMoveHandler (Variables|Default|GetDraggingCard))))

(event Custom|CustomEvent_1
  (params (location :type Vector) (screenPosition :type Vector%202D%20Structure))
  (if (Variables|Default|GetbDragging)
    (CallFunction|EndDragHandler (Variables|Default|GetDraggingCard))))

(event EventBeginPlay)

(event EventTick
  (params (DeltaSeconds :type Float%20%28single-precision%29)))

(event EventOnDrawCard
  (params (card :type Card%20Object%20Reference))
  (bind _returnvalue (Game|GetPlayerController 0))
  (bind _returnvalue_2 (Actor|GetComponentsByClass _returnvalue "/Script/Cardopoly.TouchInputDispatcherComponent"))
  (Transformation|AttachActorToActor card (Components|GetOwner self) "None" "KeepRelative" "SnapToTarget" "KeepRelative" true)
  (CallFunction|AddSlot card)
  (CallFunction|UpdateSlotsPositions)
  (CallFunction|InstantMoveCardstoPositions)
  (EventDispatchers|BindEventtoOnObjectTouchStartedDelegate _returnvalue_2 (delegate Custom|CustomEvent))
  (EventDispatchers|BindEventtoOnonTouchTriggeredDelegate _returnvalue_2 (delegate Custom|CustomEvent_0))
  (EventDispatchers|BindEventtoOnonTouchEndedDelegate _returnvalue_2 (delegate Custom|CustomEvent_1)))

(fn UpdateSlotsPositions
  (bind _bottomcenterposition (Variables|Default|GetBottomCenterPosition))
  (bind _slots (Variables|Default|GetSlots))
  (for (_array_element _array_index) (Variables|Default|GetSlots)
    (if (> (Utilities|Array|Length _slots) 1)
      (bind _structout (Utilities|Struct|SetmembersinCardSlot _array_element (Math|Vector|MakeVector (.x _bottomcenterposition) (|((((0-1)*((Length-1)/2.000000))*Distance)+(Index*Distance)) _array_index (Utilities|Array|Length (Variables|Default|GetSlots)) (Variables|Default|GetDistanceBetweenCards)) (.z _bottomcenterposition))))
      (Utilities|Array|SetArrayElem (Variables|Default|GetSlots) _array_index _structout)
      (else
        (bind _structout_2 (Utilities|Struct|SetmembersinCardSlot _array_element (Variables|Default|GetBottomCenterPosition)))
        (Utilities|Array|SetArrayElem _slots _array_index _structout_2)))))

(fn AddSlot
  (params (Card :type Card%20Object%20Reference))
  (Utilities|Array|Add (Variables|Default|GetSlots) (Utilities|Struct|MakeCardSlot Card (Math|Vector|VectorZero))))

(fn InstantMoveCardstoPositions
  (for _array_element (Variables|Default|GetSlots)
    (Transformation|SetActorRelativeLocation (.Card (Utilities|Struct|BreakCardSlot _array_element)) (.Position (Utilities|Struct|BreakCardSlot _array_element)))))

(fn CardMoveHandler
  (params (Card :type Card%20Object%20Reference))
  (bind _returnvalue (Components|GetOwner))
  (bind _returnvalue_2 (Game|GetPlayerController 0))
  (bind _returnvalue_3 (Transformation|GetActorForwardVector _returnvalue))
  (bind (_locationx _locationy) (Game|Player|GetMousePosition _returnvalue_2))
  (bind _returnvalue_4 (Math|Vector2D|MakeVector2D _locationx _locationy))
  (bind (_worldposition _worlddirection) (Class|GameplayStatics|DeprojectScreentoWorld _returnvalue_2 _returnvalue_4))
  (Transformation|SetActorRelativeLocation Card (+ (Math|Transform|InverseTransformLocation (Transformation|GetActorTransform (Components|GetOwner)) (.Intersection (Class|KismetMathLibrary|LinePlaneIntersection _worldposition (+ (* _worlddirection 5e+03) _worldposition) (Class|KismetMathLibrary|MakePlanefromPointandNormal (+ (Transformation|GetActorLocation _returnvalue) (* (.X (Math|Vector|BreakVector (Variables|Default|GetBottomCenterPosition))) _returnvalue_3)) (* _returnvalue_3 -1.0))))) (Math|Vector|MakeVector 0.0 0.0 (Variables|Default|GetCardMoveOffsetZ)))))

(fn ReturnCard
  (params (Card :type Card%20Object%20Reference))
  (for _array_element (Variables|Default|GetSlots)
    (if (== (.Card (Utilities|Struct|BreakCardSlot _array_element)) Card)
      (Class|Card|MovetoLocalPosition (.Card (Utilities|Struct|BreakCardSlot _array_element)) (.Position (Utilities|Struct|BreakCardSlot _array_element)) 0.25 "OutSine"))))

(fn RemoveCard
  (params (Card :type Card%20Object%20Reference))
  (bind _slots (Variables|Default|GetSlots))
  (LocalVariables|SetIndexToRemove -1)
  (for (_array_element _array_index) _slots
    (if (== (.Card (Utilities|Struct|BreakCardSlot _array_element)) Card)
      (LocalVariables|SetIndexToRemove _array_index)))
  (if (!= (LocalVariables|GetIndexToRemove) -1)
    (Utilities|Array|RemoveIndex _slots (LocalVariables|GetIndexToRemove))))

(fn EndDragHandler
  (params (Card :type Card%20Object%20Reference))
  (bind _returnvalue (Game|GetPlayerController 0))
  (bind (_locationx _locationy) (Game|Player|GetMousePosition _returnvalue))
  (bind _output_get (LocalVariables|SetScreenPosition (Math|Vector2D|MakeVector2D _locationx _locationy)))
  (bind _returnvalue_2 (Class|Card|CanApply Card _output_get))
  (if _returnvalue_2
    (Class|Card|Apply Card _output_get)
    (CallFunction|RemoveCard Card)
    (Variables|Default|SetDraggingCard 0)
    (Variables|Default|SetbDragging false)
    (CallFunction|UpdateSlotsPositions)
    (CallFunction|InstantMoveCardstoPositions)
    (else
      (CallFunction|ReturnCard Card)
      (Variables|Default|SetDraggingCard 0)
      (Variables|Default|SetbDragging false))))