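; RTS camera Blueprint that feeds a scene capture into a full-screen post-process material through a render target.
; On BeginPlay it creates a render target at viewport size times UpscaleMultiplier and assigns it to its SceneCaptureComponent2D.
; A dynamic material instance receives that texture and becomes the blendable on the PostProcessVolume found in the level.
; Tick detects viewport resolution changes and reruns the setup, creating a new target and material instance.
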(event EventBeginPlay
  (bind _returnvalue (Game|GetPlayerController 0))
  (bind _upscalemultiplier (Variables|Default|GetUpscaleMultiplier))
  (bind (_sizex _sizey) (HUD|GetViewportSize _returnvalue))
  (Variables|Default|SetPrevScreenResolutionX _sizex)
  (Variables|Default|SetPrevScreenResolutionY _sizey)
  (bind _returnvalue_2 (Rendering|CreateRenderTarget2D (* (Math|Conversions|ToFloat(Integer) _sizex) _upscalemultiplier) (* (Math|Conversions|ToFloat(Integer) _sizey) _upscalemultiplier) "RTF_RGBA8"))
  (bind _output_get (Variables|Default|Setrendertarget _returnvalue_2))
  (bind _returnvalue_3 (Rendering|Material|CreateDynamicMaterialInstance (Variables|Default|GetMaterial) "post_mat_inst" "None" :!class /Script/Engine.KismetMaterialLibrary))
  (Rendering|Material|SetTextureParameterValue _returnvalue_3 "Param" _output_get)
  (bind _returnvalue_4 (Actor|GetActorOfClass "/Script/Engine.PostProcessVolume"))
  (bind _structout (Utilities|Struct|SetmembersinPostProcessSettings (Variables|/Script/Engine.PostProcessVolume|GetSettings _returnvalue_4) (Utilities|Struct|MakeWeightedBlendables (Utilities|Array|MakeArray (Utilities|Struct|MakeWeightedBlendable 1.0 _returnvalue_3)))))
  (Variables|/Script/Engine.SceneCaptureComponent2D|SetTextureTarget (Actor|GetComponentbyClass "/Script/Engine.SceneCaptureComponent2D") _output_get)
  (Variables|/Script/Engine.PostProcessVolume|SetSettings _returnvalue_4 _structout))

(event Collision|EventActorBeginOverlap
  (params (OtherActor :type Actor%20Object%20Reference)))

(event EventTick
  (params (DeltaSeconds :type Float%20%28single-precision%29))
  (bind _returnvalue (Game|GetPlayerController 0))
  (bind _upscalemultiplier (Variables|Default|GetUpscaleMultiplier))
  (bind (_sizex _sizey) (HUD|GetViewportSize _returnvalue))
  (if (or (!= _sizex (Variables|Default|GetPrevScreenResolutionX)) (!= _sizey (Variables|Default|GetPrevScreenResolutionY)))
    (Variables|Default|SetPrevScreenResolutionX _sizex)
    (Variables|Default|SetPrevScreenResolutionY _sizey)
    (bind _returnvalue_2 (Rendering|CreateRenderTarget2D (* (Math|Conversions|ToFloat(Integer) _sizex) _upscalemultiplier) (* (Math|Conversions|ToFloat(Integer) _sizey) _upscalemultiplier) "RTF_RGBA8"))
    (bind _output_get (Variables|Default|Setrendertarget _returnvalue_2))
    (bind _returnvalue_3 (Rendering|Material|CreateDynamicMaterialInstance (Variables|Default|GetMaterial) "post_mat_inst" "None" :!class /Script/Engine.KismetMaterialLibrary))
    (Rendering|Material|SetTextureParameterValue _returnvalue_3 "Param" _output_get)
    (bind _returnvalue_4 (Actor|GetActorOfClass "/Script/Engine.PostProcessVolume"))
    (bind _structout (Utilities|Struct|SetmembersinPostProcessSettings (Variables|/Script/Engine.PostProcessVolume|GetSettings _returnvalue_4) (Utilities|Struct|MakeWeightedBlendables (Utilities|Array|MakeArray (Utilities|Struct|MakeWeightedBlendable 1.0 _returnvalue_3)))))
    (Variables|/Script/Engine.SceneCaptureComponent2D|SetTextureTarget (Actor|GetComponentbyClass "/Script/Engine.SceneCaptureComponent2D") _output_get)
    (Variables|/Script/Engine.PostProcessVolume|SetSettings _returnvalue_4 _structout)))

(fn ConstructionScript)